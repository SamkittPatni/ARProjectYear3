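; WorldLocationReference is an actor that moves according to the VR pawn's headset position.
; BeginPlay stores the VRPawn's HMD X and Y with a fixed height as LastLocation.
; Each Tick adds the difference between the current HMD position and LastLocation as a local-space offset, without sweeping.
; LastLocation is never updated after BeginPlay, so the offset accumulates every frame the headset is away from its starting point.
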(event EventBeginPlay
  (bind _returnvalue (Actor|GetActorOfClass "/Game/Blueprints/VRPawn2.VRPawn_C"))
  (bind _hmdlocation (Default|GetHMDLocation _returnvalue))
  (Variables|Default|SetLastLocation (Math|Vector|MakeVector (.X (Class|KismetMathLibrary|BreakVector3f _hmdlocation)) (.Y (Class|KismetMathLibrary|BreakVector3f _hmdlocation)) 1.9e+02)))

(event Collision|EventActorBeginOverlap
  (params (OtherActor :type Actor%20Object%20Reference)))

(event EventTick
  (params (DeltaSeconds :type Float%20%28single-precision%29))
  (bind _returnvalue (Actor|GetActorOfClass "/Game/Blueprints/VRPawn2.VRPawn_C"))
  (bind _hmdlocation (Default|GetHMDLocation _returnvalue))
  (Transformation|AddActorLocalOffset (- (Math|Vector|MakeVector (.X (Class|KismetMathLibrary|BreakVector3f _hmdlocation)) (.Y (Class|KismetMathLibrary|BreakVector3f _hmdlocation)) 1.9e+02) (Variables|Default|GetLastLocation)) false false))

(fn ConstructionScript)