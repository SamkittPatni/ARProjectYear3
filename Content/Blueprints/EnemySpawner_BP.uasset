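; Enemy spawner that keeps the EnemyAI_BP population topped up to EnemyAmount.
; After a startup delay, a BeginPlay loop spawns enemies back to back, rechecking after a delay once at the cap.
; Spawns use random points in FloorPlane_BP bounds, raised and yawed toward world X/Y zero, then SetWorldTransform reapplies the random-point expression.
; Tick zeroes EnemyAmount when the first VRPawn's health runs out, halting spawns.
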(event EventBeginPlay
  (Variables|Default|SetBeginPlay false)
  (Utilities|FlowControl|Delay 5.0)
  (bind _outactors (Actor|GetAllActorsOfClass "/Game/Blueprints/EnemyAI_BP.EnemyAI_BP_C" :!label _label))
  (if (>= (Utilities|Array|Length _outactors) (Variables|Default|Getenemy_amount))
    (Utilities|FlowControl|Delay 5.0)
    (goto _label)
    (else
      (bind _returnvalue (Actor|GetActorOfClass "/Game/Blueprints/FloorPlane_BP.FloorPlane_BP_C"))
      (bind _returnvalue_2 (Game|SpawnActorfromClass "/Game/Blueprints/EnemyAI_BP.EnemyAI_BP_C" (Math|Transform|MakeTransform (Math|Vector|MakeVector (.X (Class|KismetMathLibrary|BreakVector3f (.Location (Math|Transform|BreakTransform (Math|Conversions|ToTransform(Vector) (Math|Random|RandomPointinBoundingBox (.Origin (Collision|GetActorBounds _returnvalue false false)) (.BoxExtent (Collision|GetActorBounds _returnvalue false false)))))))) (.Y (Class|KismetMathLibrary|BreakVector3f (.Location (Math|Transform|BreakTransform (Math|Conversions|ToTransform(Vector) (Math|Random|RandomPointinBoundingBox (.Origin (Collision|GetActorBounds _returnvalue false false)) (.BoxExtent (Collision|GetActorBounds _returnvalue false false)))))))) (+ (.Z (Class|KismetMathLibrary|BreakVector3f (.Location (Math|Transform|BreakTransform (Math|Conversions|ToTransform(Vector) (Math|Random|RandomPointinBoundingBox (.Origin (Collision|GetActorBounds _returnvalue false false)) (.BoxExtent (Collision|GetActorBounds _returnvalue false false)))))))) 2.8e+02)) (Math|Rotator|FindLookatRotation (Math|Vector|MakeVector (.X (Class|KismetMathLibrary|BreakVector3f (.Location (Math|Transform|BreakTransform (Math|Conversions|ToTransform(Vector) (Math|Random|RandomPointinBoundingBox (.Origin (Collision|GetActorBounds _returnvalue false false)) (.BoxExtent (Collision|GetActorBounds _returnvalue false false)))))))) (.Y (Class|KismetMathLibrary|BreakVector3f (.Location (Math|Transform|BreakTransform (Math|Conversions|ToTransform(Vector) (Math|Random|RandomPointinBoundingBox (.Origin (Collision|GetActorBounds _returnvalue false false)) (.BoxExtent (Collision|GetActorBounds _returnvalue false false)))))))) (+ (.Z (Class|KismetMathLibrary|BreakVector3f (.Location (Math|Transform|BreakTransform (Math|Conversions|ToTransform(Vector) (Math|Random|RandomPointinBoundingBox (.Origin (Collision|GetActorBounds _returnvalue false false)) (.BoxExtent (Collision|GetActorBounds _returnvalue false false)))))))) 2.8e+02)) (Math|Vector|MakeVector 0.0 0.0 (+ (.Z (Class|KismetMathLibrary|BreakVector3f (.Location (Math|Transform|BreakTransform (Math|Conversions|ToTransform(Vector) (Math|Random|RandomPointinBoundingBox (.Origin (Collision|GetActorBounds _returnvalue false false)) (.BoxExtent (Collision|GetActorBounds _returnvalue false false)))))))) 2.8e+02)))) "AdjustIfPossibleButAlwaysSpawn" 0 0))
      (Transformation|SetWorldTransform (Variables|/Script/Engine.Actor|GetRootComponent _returnvalue_2) (Math|Transform|MakeTransform (Math|Vector|MakeVector (.X (Class|KismetMathLibrary|BreakVector3f (.Location (Math|Transform|BreakTransform (Math|Conversions|ToTransform(Vector) (Math|Random|RandomPointinBoundingBox (.Origin (Collision|GetActorBounds _returnvalue false false)) (.BoxExtent (Collision|GetActorBounds _returnvalue false false)))))))) (.Y (Class|KismetMathLibrary|BreakVector3f (.Location (Math|Transform|BreakTransform (Math|Conversions|ToTransform(Vector) (Math|Random|RandomPointinBoundingBox (.Origin (Collision|GetActorBounds _returnvalue false false)) (.BoxExtent (Collision|GetActorBounds _returnvalue false false)))))))) (+ (.Z (Class|KismetMathLibrary|BreakVector3f (.Location (Math|Transform|BreakTransform (Math|Conversions|ToTransform(Vector) (Math|Random|RandomPointinBoundingBox (.Origin (Collision|GetActorBounds _returnvalue false false)) (.BoxExtent (Collision|GetActorBounds _returnvalue false false)))))))) 2.8e+02)) (Math|Rotator|FindLookatRotation (Math|Vector|MakeVector (.X (Class|KismetMathLibrary|BreakVector3f (.Location (Math|Transform|BreakTransform (Math|Conversions|ToTransform(Vector) (Math|Random|RandomPointinBoundingBox (.Origin (Collision|GetActorBounds _returnvalue false false)) (.BoxExtent (Collision|GetActorBounds _returnvalue false false)))))))) (.Y (Class|KismetMathLibrary|BreakVector3f (.Location (Math|Transform|BreakTransform (Math|Conversions|ToTransform(Vector) (Math|Random|RandomPointinBoundingBox (.Origin (Collision|GetActorBounds _returnvalue false false)) (.BoxExtent (Collision|GetActorBounds _returnvalue false false)))))))) (+ (.Z (Class|KismetMathLibrary|BreakVector3f (.Location (Math|Transform|BreakTransform (Math|Conversions|ToTransform(Vector) (Math|Random|RandomPointinBoundingBox (.Origin (Collision|GetActorBounds _returnvalue false false)) (.BoxExtent (Collision|GetActorBounds _returnvalue false false)))))))) 2.8e+02)) (Math|Vector|MakeVector 0.0 0.0 (+ (.Z (Class|KismetMathLibrary|BreakVector3f (.Location (Math|Transform|BreakTransform (Math|Conversions|ToTransform(Vector) (Math|Random|RandomPointinBoundingBox (.Origin (Collision|GetActorBounds _returnvalue false false)) (.BoxExtent (Collision|GetActorBounds _returnvalue false false)))))))) 2.8e+02)))) false false)
      (goto _label))))

(event Collision|EventActorBeginOverlap
  (params (OtherActor :type Actor%20Object%20Reference)))

(event EventTick
  (params (DeltaSeconds :type Float%20%28single-precision%29))
  (bind _outactors (Actor|GetAllActorsOfClass "/Game/Blueprints/VRPawn2.VRPawn_C"))
  (if (<= (Variables|/Game/Blueprints/VRPawn2.VRPawn_C|GetPlayerHealth (Utilities|Array|Get(acopy) _outactors)) 0.0)
    (Variables|Default|Setenemy_amount 0)))

(fn ConstructionScript)