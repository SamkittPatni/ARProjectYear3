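; Sword-wielding melee enemy that chases a pawn spotted by PawnSensing via AIMoveTo and attacks on arrival.
; Attacks use animations and delays gated by CanHit and CanDamage; the sword line trace draws debug but its result is unused when applying damage.
; Any actor overlap costs HitPoints, plays a hit reaction and briefly disables collision and damage output.
; Tick destroys it at zero health or after falling too low.
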(event OnSeePawn(PawnSensing)
  (params (Pawn :type Pawn%20Object%20Reference))
  (Variables|Default|SetisSeeingPlayer true)
  (CallFunction|FollowPlayer))

(event Custom|FollowPlayer
  (bind _sword (Variables|Default|Getsword))
  (if (Variables|Default|GetisSeeingPlayer)
    (AI|AIMoveTo self "0, 0, 0" (stale OnSeePawn(PawnSensing) Pawn) 1.2e+02 false
      (:OnSuccess
        (if (Variables|Default|GetcanHit)
          (Variables|Default|SetcanHit false)
          (Components|Animation|PlayAnimation (Variables|Character|GetMesh) "/Game/Anim_Sword_1H_Attack_Slash2.Anim_Sword_1H_Attack_Slash2" false)
          (bind _outhit (Collision|LineTraceByChannel (Transformation|GetSocketLocation _sword "start") (Transformation|GetSocketLocation _sword "end") "TraceTypeQuery2" false 0 "Persistent" true "(R=1.000000,G=0.000000,B=0.000000,A=1.000000)" "(R=0.000000,G=1.000000,B=0.000000,A=1.000000)" 1.03))
          (Utilities|FlowControl|Delay 0.9)
          (if (Variables|Default|GetcanDamage)
            (Game|Damage|ApplyDamage (stale OnSeePawn(PawnSensing) Pawn) 2e+01 0 0))
          (Components|Animation|PlayAnimation (Variables|Character|GetMesh) "/Game/Anim_Sword_1H_Laydown.Anim_Sword_1H_Laydown" false)
          (Utilities|FlowControl|Delay 1.1)
          (Variables|Default|SetcanHit true))))))

(event EventBeginPlay
  (Variables|Default|SetcanHit true)
  (Variables|Default|SetcanDamage true))

(event Collision|EventActorBeginOverlap
  (params (OtherActor :type Actor%20Object%20Reference))
  (Variables|Default|SetHitPoints (- (Variables|Default|GetHitPoints) 1e+02))
  (Collision|SetCollisionEnabled (Variables|Character|GetMesh) "NoCollision")
  (Collision|SetCollisionEnabled (Variables|Collision|GetCapsuleComponent) "NoCollision")
  (Components|Animation|PlayAnimation (Variables|Character|GetMesh) "/Game/Anim_Sword_1H_Big_Hit_Front.Anim_Sword_1H_Big_Hit_Front" false)
  (Variables|Default|SetcanDamage false)
  (Utilities|FlowControl|Delay 1.5)
  (Collision|SetCollisionEnabled (Variables|Character|GetMesh) "QueryOnly")
  (Collision|SetCollisionEnabled (Variables|Collision|GetCapsuleComponent) "QueryOnly")
  (Variables|Default|SetcanDamage true))

(event EventTick
  (params (DeltaSeconds :type Float%20%28single-precision%29))
  (if (or (<= (Variables|Default|GetHitPoints) 0.0) (< (.Z (Class|KismetMathLibrary|BreakVector3f (Transformation|GetActorLocation))) -1e+03))
    (Actor|DestroyActor)))

(fn ConstructionScript)